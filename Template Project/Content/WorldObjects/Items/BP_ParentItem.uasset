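; BP_ParentItem is the parent Blueprint for world items, declaring hooks for pickup, dropping, storage attachment, conveyors, highlighting, clicks and physics locking.
; Nearly all events and functions are empty here, including the scan functions and construction script.
; The implemented logic is conveyor movement: a loop function overwrites the mesh's physics velocity along a direction vector, scaled by clamped water pressure.
; A companion function clears all stored conveyor timers.
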(event Custom|ItemPickedUp
  (params (Player :type BP%20Game%20Character%20Object%20Reference)))

(event Custom|AutoLock)

(event Custom|EnteredConveyor
  (params (Collision%20Comp :type Actor%20Component%20Object%20Reference) (VecDirection :type Vector) (WaterPressure :type Float%20%28single-precision%29) (LockOut? :type Boolean)))

(event Custom|OverrideRightClickIsTarget
  (params (Component :type Primitive%20Component%20Object%20Reference)))

(event Custom|TriggerTypeBLock)

(event Custom|TryAttachToStorage
  (params (BeingStoredBy :type Actor%20Object%20Reference) (Component :type Scene%20Component%20Object%20Reference)))

(event Custom|TypeBPhysicsLock)

(event Custom|StorageLoop)

(event Custom|OverrideClickNoTarget
  (params (Controller :type BP%20Game%20Controller%20Object%20Reference) (Hit%20Actor :type Actor%20Object%20Reference)))

(event Custom|OverrideUnhighlighted)

(event Custom|OverrideLockedPhysics)

(event Custom|OverrideHighlighted)

(event Custom|OverrideMouseActivated
  (params (Component :type Primitive%20Component%20Object%20Reference)))

(event Custom|OverrideStopClicking)

(event Custom|ItemFreeDropping
  (params (Player :type BP%20Game%20Character%20Object%20Reference)))

(event Custom|DetachFromStorage)

(event Custom|FlashRedTimer)

(event Custom|OverridePickedup)

(event Custom|OverrideLoaded)

(event Custom|OverrideRightClickNoTarget)

(event Custom|OverrideDroppedItem)

(event Custom|OverrideInWater)

(event Custom|ItemDropped)

(event Custom|FlashRed)

(event Custom|ExitConveyor
  (params (Collision%20Comp :type Actor%20Component%20Object%20Reference) (RemoveLockout :type Boolean)))

(event Custom|AttachToStorage
  (params (Storage :type Actor%20Object%20Reference) (MeshToAttachTo :type Scene%20Component%20Object%20Reference) (Channel :type ECollisionChannel%20Enum :default "ECC_WorldStatic")))

(event Custom|LerpToCharacter
  (params (Component :type Scene%20Component%20Object%20Reference)))

(fn ConstructionScript)

(fn ScanforItems)

(fn ScanforDropCollision)

(fn SetAdditionalMeshesNewResponse)

(fn ConveyorTimerLoop
  (Class|PrimitiveComponent|SetAllPhysicsLinearVelocity (Variables|Default|GetStaticMesh) (* (Variables|Default|GetDirectionalVector) (Math|Float|MapRangeClamped (Variables|Default|GetWaterPressure) 1.0 1e+02 1e+02 1.5e+02)) false))

(fn ClearConveyorTimers
  (bind _conveyortimerhandles (Variables|Default|GetConveyorTimerHandles))
  (for _array_element _conveyortimerhandles
    (Utilities|Time|ClearandInvalidateTimerbyHandle _array_element))
  (Utilities|Array|Clear _conveyortimerhandles))